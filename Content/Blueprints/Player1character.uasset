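; Player 1 character for a 2D side-view game, with horizontal movement, jumping and flipbook animation.
; MoveRight and Moveleft axes both add movement along world X, and the Jump action starts and stops jumping.
; Each tick picks a fall, run or idle flipbook from falling state and speed.
; It also flips controller yaw between 0 and 180 by X velocity to face the direction of travel.
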(event `self.ReceiveTick`
  (params (DeltaSeconds :type "Float (single-precision)"))
  ;[1 1 1] Update Sprite animation
  (`self.Uptade Animation`)
  (`self.UpdateControlRotation`))

(event `InputAxis|MoveRight`
  (params (AxisValue :type "Float (single-precision)"))
  ;[1 1 1] Movimento Direita/Esquerda e Pulo
  (`self.AddMovementInput` (0.5 0.0 0.0) AxisValue))

(event `Uptade Animation`
  ;[1 1 1] Função Update animation
  (`PaperFlipbookComponent.SetFlipbook` (`self.Sprite`) (select `bool` (`NavMovementComponent.IsFalling` (`self.CharacterMovement`)) :`false` (select `bool` (> (`KismetMathLibrary.VSize` (`MovementComponent.Velocity` (`self.CharacterMovement`))) 0.0) :`false` "/Game/Sprites/herochar_sprites_new_/Idle_animation/player_idle.player_idle" :`true` "/Game/Sprites/herochar_sprites_new_/run_animation/run_animationplayer1.run_animationplayer1" :!type "PaperFlipbook Object Reference") :`true` "/Game/Sprites/herochar_sprites_new_/jumpdown/fallanimation.fallanimation")))

(event `InputAxis|Moveleft`
  (params (AxisValue :type "Float (single-precision)"))
  ;[1 1 1] Movimento Direita/Esquerda e Pulo
  (`self.AddMovementInput` (0.5 0.0 0.0) AxisValue))

(event `InputAction|Jump`
  (params (Key :type "Key Structure"))
  ;[1 1 1] Movimento Direita/Esquerda e Pulo
  (:`Pressed`
    (`self.Jump`))
  (:`Released`
    (`self.StopJumping`)))

(event `UpdateControlRotation`
  ;[1 1 1] Função rotação da animação
  (`/Engine/EditorBlueprintResources/StandardMacros.IsValid` (`self.GetController`)
    (:`Is Valid`
      (`/Engine/EditorBlueprintResources/StandardMacros.CompareFloat` (.x (`MovementComponent.Velocity` (`self.CharacterMovement`)))
        (:`>`
          (`Controller.SetControlRotation` (`self.GetController`) (`KismetMathLibrary.MakeRotator` 0.0)))
        (:`<`
          (`Controller.SetControlRotation` (`self.GetController`) (`KismetMathLibrary.MakeRotator` 0.0 0.0 180.0)))))))

(fn `UserConstructionScript`)